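; Boss dragon enemy with its own HUD and HP; depleting it shows the win screen and pauses the game.
; Checkhit plays attack sounds and sends OnhitMessage to the cached target within range of the Fire component's socket.
; When that target is invalid, a sphere trace picks a Pawn; its nearest-enemy comparison measures the same distance twice, so the last hit wins.
; OnhitD applies fixed damage to the dragon.
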(event EventBeginPlay)

(event Collision|EventActorBeginOverlap
  (params (OtherActor :type Actor%20Object%20Reference)))

(event EventTick
  (params (DeltaSeconds :type Float%20%28single-precision%29)))

(event EventOnhitD
  ;[1 1 1] Update when player hit dragon
  (bind _output_get (Variables|Default|SetHP (- (Variables|Default|GetHP) 25.0)))
  (if (<= _output_get 0.0)
    (bind _returnvalue (UserInterface|CreateWidget "/Game/Widgets/WinLose.WinLose_C" (Game|GetPlayerController 0) "You Win!"))
    (UserInterface|Viewport|AddtoViewport _returnvalue 0)
    (Game|SetGamePaused true)))

(event EventBeginPlay
  ;[1 1 1] Create hud widget for dragon
  (Variables|Default|SetHP 5e+02)
  (bind _returnvalue (UserInterface|CreateWidget "/Game/Widgets/HUD_Dragon.HUD_Dragon_C" (Game|GetPlayerController 0) self))
  (UserInterface|Viewport|AddtoViewport _returnvalue 0))

(event EventCheckhit
  (bind _nearest_enemy (Variables|Default|GetNearest%20Enemy))
  ;[1 1 1] Update when dragon hit around
  (Audio|PlaySoundatLocation "/Game/Sound/195937__michimuc2__short-wind-noise_Cue.195937__michimuc2__short-wind-noise_Cue" "0, 0, 0" "0, 0, 0" 1.0 1.0 0.0 0 0 0)
  (Utilities|IsValid _nearest_enemy
    (:Is%20Valid
      _)
    (:Is%20Not%20Valid
      (CallFunction|GetNearestEnemy)))
  (Utilities|IsValid _nearest_enemy
    (:Is%20Valid
      (if (< (Math|Vector|VectorLength (- (Transformation|GetSocketLocation (Variables|Default|GetFire) "CubeSocket") (Transformation|GetActorLocation _nearest_enemy))) (Variables|Default|GetHit%20Range))
        (Audio|PlaySoundatLocation "/Game/Sound/326810__johnbuhr__sword-clash-32__1__Cue.326810__johnbuhr__sword-clash-32__1__Cue" "0, 0, 0" "0, 0, 0" 1.0 1.0 0.0 0 0 0)
        (Class|BPInterfaceTy|Onhit(Message) (Variables|Default|GetNearest%20Enemy))))))

(fn ConstructionScript)

(fn GetNearestEnemy
  (bind _returnvalue (Transformation|GetActorLocation))
  (bind _self self)
  (bind (_x _y _z) (Math|Vector|BreakVector _returnvalue))
  (bind _outhits (Collision|MultiSphereTraceForObjects _returnvalue (Math|Vector|MakeVector (+ _x 1e+02) (+ _y 1e+02) (+ _z 1e+02)) 2e+02 (Utilities|Array|MakeArray "ObjectTypeQuery3") false 0 "None"))
  (for _array_element _outhits
    (Utilities|IsValid (Variables|Default|GetNearest%20Enemy)
      (:Is%20Valid
        (if (not (< (Transformation|GetDistanceTo (Variables|Default|GetNearest%20Enemy) _self) (Transformation|GetDistanceTo _self (Variables|Default|GetNearest%20Enemy))))
          (Variables|Default|SetNearest%20Enemy (.hitactor _array_element) :!label _label)))
      (:Is%20Not%20Valid
        (goto _label))))
  (return (Variables|Default|GetNearest%20Enemy)))