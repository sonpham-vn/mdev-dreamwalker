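; Trigger box that flags a BP_Base actor as inside Zone1 and lets the player trigger a notification sound with the talk input.
; Overlap enables input, sets Zone1 and opens a Gate, so each talk press plays the station notification cue at the world origin.
; Ending overlap disables input and clears Zone1 but leaves the Gate open.
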(event EventBeginPlay)

(event Collision|EventActorBeginOverlap
  (params (OtherActor :type Actor%20Object%20Reference))
  (Input|EnableInput (Game|GetPlayerController 0))
  (bind _asbp_base (Utilities|Casting|CastToBP_Base OtherActor))
  (Variables|/Game/Blueprints/BP_Base.BP_Base_C|Setzone1 _asbp_base true)
  (Utilities|FlowControl|Gate true) ; enters at Open
)

(event EventTick
  (params (DeltaSeconds :type Float%20%28single-precision%29)))

(event Collision|EventActorEndOverlap
  (params (OtherActor :type Actor%20Object%20Reference))
  (Input|DisableInput (Game|GetPlayerController 0))
  (bind _asbp_base (Utilities|Casting|CastToBP_Base OtherActor))
  (Variables|/Game/Blueprints/BP_Base.BP_Base_C|Setzone1 _asbp_base false))

(event Input|ActionEvents|InputActiontalk
  (params (Key :type Key%20Structure :default "None"))
  (:Pressed
    (Utilities|FlowControl|Gate true
      (:Exit
        (Audio|PlaySoundatLocation "/Game/Sound/Station_Notification_Cue.Station_Notification_Cue" "0, 0, 0" "0, 0, 0" 1.0 1.0 0.0 0 0 0)))))

(fn ConstructionScript)